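; Floating text actor that raises its TextRender and then destroys itself.
; BeginPlay starts a MoveComponentTo over TimeFloating, targeting 200 units above the text's world location, passed as a relative location.
; SetUpFloatingText sets the duration and restarts the float only when DontDestoy is false, otherwise doing nothing.
; DestroyActor follows the move unconditionally, as the DontDestoyText check is disconnected.
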(event Custom|SetUpFloatingText
  (params (DurationLife :type Float%20%28double-precision%29) (DontDestoy :type Boolean))
  (if (not DontDestoy)
    (Variables|Default|SetTimeFloating DurationLife)
    (Variables|Default|SetDontDestoyText DontDestoy)
    (CallFunction|StartFloating)))

(event Custom|StartFloating
  (bind _textrender (Variables|Default|GetTextRender))
  (bind _returnvalue (Transformation|GetWorldLocation _textrender))
  (Components|MoveComponentTo (Variables|Default|GetTextRender) (Math|Vector|MakeVector (.x _returnvalue) (.y _returnvalue) (+ (.z _returnvalue) 2e+02)) "0, 0, 0" false false (Variables|Default|GetTimeFloating) false)
  (Actor|DestroyActor))

(event EventBeginPlay
  (CallFunction|StartFloating))

(fn ConstructionScript)