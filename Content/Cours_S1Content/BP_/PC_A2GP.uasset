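; Player controller that handles Enhanced Input for the player character: movement, look, jump, crouch, sprint and camera switching.
; It creates the HUD on BeginPlay and opens its inventory and pause menus from input.
; Sprinting raises walk speed, while looping timers drain stamina during movement and regenerate it after a delay once sprint stops or stamina empties.
; Run and walk states send camera messages to the character to adjust arm length and offset.
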(event Custom|UseStamina
  ;[0.03529 0.03529 0.03529] RUN AND STAMINA
  (if (Variables|Default|GetIsMoving)
    (Variables|Default|SetStamina (Math|Float|Clamp(Float) (- (Variables|Default|GetStamina) 0.5) 0.0 1e+02))
    (if (== (Variables|Default|GetStamina) 0.0)
      (Utilities|Time|ClearandInvalidateTimerbyHandle (Variables|Default|GetStaminaSpendTimeHandle))
      (CallFunction|RegenStam)
      (else
        (CallFunction|RunCamera)))
    (else
      (CallFunction|WalkCamera))))

(event Custom|IncreaseStamina
  ;[0.03529 0.03529 0.03529] RUN AND STAMINA
  (if (!= (Variables|Default|GetIsRun) true)
    (Variables|Default|SetStamina (Math|Float|Clamp(Float) (+ (Variables|Default|GetStamina) 3.0) 0.0 1e+02))
    (Development|PrintString (Utilities|String|ToString(Float) (Variables|Default|GetStamina)))
    (if (== (Variables|Default|GetStamina) 1e+02)
      (Utilities|Time|ClearandInvalidateTimerbyHandle (Variables|Default|GetStaminaRegenTimeHandle)))))

(event Custom|RegenStam
  ;[0.03529 0.03529 0.03529] RUN AND STAMINA
  (Variables|/Script/Engine.CharacterMovementComponent|SetMaxWalkSpeed (Variables|Default|GetCharacterMovement) 2.5e+02)
  (Utilities|Time|ClearandInvalidateTimerbyHandle (Variables|Default|GetStaminaSpendTimeHandle))
  (bind _returnvalue (Utilities|Time|SetTimerbyEvent (delegate Custom|IncreaseStamina) 1.0 true (Variables|Default|GetDelayRegen)))
  (Variables|Default|SetStaminaRegenTimeHandle _returnvalue)
  (CallFunction|WalkCamera))

(event Custom|RunCamera
  (Class|CameraInterface|CameraMove(Message) (Variables|Default|GetPlayerCharacter) 175.0 2e+01)
  (Class|CameraInterface|CameraReset(Message) (Variables|Default|GetPlayerCharacter)))

(event Custom|WalkCamera
  (bind _playercharacter (Variables|Default|GetPlayerCharacter))
  (Class|CameraInterface|CameraMove(Message) _playercharacter 1e+02 35.0)
  (Class|CameraInterface|CameraReset(Message) _playercharacter))

(event Input|EnhancedActionEvents|EnhancedInputActionIA_jump
  (params (ActionValue :type Boolean) (ElapsedSeconds :type Float%20%28double-precision%29) (TriggeredSeconds :type Float%20%28double-precision%29) (InputAction :type Input%20Action%20Object%20Reference :default "/Game/Cours_S1Content/Input/IA_/IA_jump.IA_jump"))
  (bind _playercharacter (Variables|Default|GetPlayerCharacter))
  (:Started
    (Character|Jump _playercharacter))
  (:Completed
    (Character|StopJumping _playercharacter)))

(event Input|EnhancedActionEvents|EnhancedInputActionIA_Move
  (params (ActionValue :type Vector%202D%20Structure) (ElapsedSeconds :type Float%20%28double-precision%29) (TriggeredSeconds :type Float%20%28double-precision%29) (InputAction :type Input%20Action%20Object%20Reference :default "/Game/Cours_S1Content/Input/IA_/IA_Move.IA_Move"))
  (bind _returnvalue (Game|Player|GetPlayerPawn 0))
  (bind _returnvalue_2 (Game|Player|GetPlayerPawn 0))
  (bind _returnvalue_3 (Pawn|GetControlRotation _returnvalue_2 :!class /Script/Engine.Pawn))
  ;[0.03529 0.03529 0.03529] Moving
  (:Triggered
    (Variables|Default|Setx (.x ActionValue))
    (Variables|Default|Sety (.y ActionValue))
    (Pawn|Input|AddMovementInput _returnvalue_2 (Math|Vector|GetRightVector (Math|Rotator|MakeRotator (.roll _returnvalue_3) 0.0 (.yaw _returnvalue_3))) (Variables|Default|Getx) false)
    (Pawn|Input|AddMovementInput _returnvalue (Math|Vector|GetForwardVector (Math|Rotator|MakeRotator 0.0 0.0 (.yaw (Pawn|GetControlRotation _returnvalue :!class /Script/Engine.Pawn)))) (Variables|Default|Gety) false))
  (:Started
    (Variables|Default|SetIsMoving true))
  (:Completed
    (Variables|Default|SetIsMoving false)))

(event Input|EnhancedActionEvents|EnhancedInputActionIA_Run
  (params (ActionValue :type Boolean) (ElapsedSeconds :type Float%20%28double-precision%29) (TriggeredSeconds :type Float%20%28double-precision%29) (InputAction :type Input%20Action%20Object%20Reference :default "/Game/Cours_S1Content/Input/IA_/IA_Run.IA_Run"))
  ;[0.03529 0.03529 0.03529] RUN AND STAMINA
  (bind _output_get (Variables|Default|SetIsRun ActionValue))
  (if _output_get
    (if (!= (Variables|Default|GetStamina) 0.0)
      (Variables|/Script/Engine.CharacterMovementComponent|SetMaxWalkSpeed (Variables|Default|GetCharacterMovement) 5e+02)
      (Utilities|Time|ClearandInvalidateTimerbyHandle (Variables|Default|GetStaminaRegenTimeHandle))
      (bind _returnvalue (Utilities|Time|SetTimerbyEvent (delegate Custom|UseStamina) 0.1 true))
      (Variables|Default|SetStaminaSpendTimeHandle _returnvalue)
      (else
        (CallFunction|WalkCamera)))
    (else
      (Variables|/Script/Engine.CharacterMovementComponent|SetMaxWalkSpeed (Variables|Default|GetCharacterMovement) 2.5e+02)
      (Utilities|Time|ClearandInvalidateTimerbyHandle (Variables|Default|GetStaminaSpendTimeHandle))
      (bind _returnvalue_2 (Utilities|Time|SetTimerbyEvent (delegate Custom|IncreaseStamina) 1.0 true (Variables|Default|GetDelayRegen)))
      (Variables|Default|SetStaminaRegenTimeHandle _returnvalue_2)
      (CallFunction|WalkCamera))))

(event Input|EnhancedActionEvents|EnhancedInputActionIA_Look
  (params (ActionValue :type Vector%202D%20Structure) (ElapsedSeconds :type Float%20%28double-precision%29) (TriggeredSeconds :type Float%20%28double-precision%29) (InputAction :type Input%20Action%20Object%20Reference :default "/Game/Cours_S1Content/Input/IA_/IA_Look.IA_Look"))
  (bind _returnvalue (Game|Player|GetPlayerPawn 0))
  (Pawn|Input|AddControllerYawInput _returnvalue (.x ActionValue))
  (Pawn|Input|AddControllerPitchInput _returnvalue (.y ActionValue)))

(event Input|EnhancedActionEvents|EnhancedInputActionIA_Pause
  (params (ActionValue :type Boolean) (ElapsedSeconds :type Float%20%28double-precision%29) (TriggeredSeconds :type Float%20%28double-precision%29) (InputAction :type Input%20Action%20Object%20Reference :default "/Game/Cours_S1Content/Input/IA_/IA_Pause.IA_Pause"))
  (bind _hud (Variables|Default|GetHUD))
  (:Started
    (Default|DisplayPlayerMenu _hud)
    (Default|OpenUIPause _hud)))

(event Input|EnhancedActionEvents|EnhancedInputActionIA_Crouch
  (params (ActionValue :type Boolean) (ElapsedSeconds :type Float%20%28double-precision%29) (TriggeredSeconds :type Float%20%28double-precision%29) (InputAction :type Input%20Action%20Object%20Reference :default "/Game/Cours_S1Content/Input/IA_/IA_Crouch.IA_Crouch"))
  (bind _playercharacter (Variables|Default|GetPlayerCharacter))
  (if ActionValue
    (Character|Crouch _playercharacter)
    (Development|PrintString "is crouch")
    (else
      (Character|UnCrouch _playercharacter)
      (Development|PrintString "not  crouch"))))

(event Input|EnhancedActionEvents|EnhancedInputActionIA_ChangeCamera
  (params (ActionValue :type Boolean) (ElapsedSeconds :type Float%20%28double-precision%29) (TriggeredSeconds :type Float%20%28double-precision%29) (InputAction :type Input%20Action%20Object%20Reference :default "/Game/Cours_S1Content/Input/IA_/IA_ChangeCamera.IA_ChangeCamera"))
  (:Started
    (Class|CameraInterface|CameraChange(Message) (Variables|Default|GetPlayerCharacter))))

(event Input|EnhancedActionEvents|EnhancedInputActionIA_Inventory
  (params (ActionValue :type Boolean) (ElapsedSeconds :type Float%20%28double-precision%29) (TriggeredSeconds :type Float%20%28double-precision%29) (InputAction :type Input%20Action%20Object%20Reference :default "/Game/Cours_S1Content/Input/IA_/IA_Inventory.IA_Inventory"))
  (bind _hud (Variables|Default|GetHUD))
  (:Started
    (Default|DisplayPlayerMenu _hud)
    (Default|OpenUIInventory _hud)))

(event EventBeginPlay
  (bind _returnvalue (Game|GetPlayerCharacter 0))
  (Utilities|FlowControl|Sequence
    (:then_0
      (Variables|Default|SetCharacterMovement (Variables|/Script/Engine.Character|GetCharacterMovement _returnvalue))
      (Variables|Default|SetPlayerCharacter _returnvalue))
    (:then_1
      (bind _returnvalue_2 (UserInterface|CreateWidget "/Game/Cours_S1Content/UI/Wb_PlayerHUD.Wb_PlayerHUD_C"))
      (bind _output_get (Variables|Default|SetHUD _returnvalue_2))
      (UserInterface|Viewport|AddtoViewport _output_get 0))
    (:then_2
      (Variables|/Script/Engine.CharacterMovementComponent|SetMaxWalkSpeed (Variables|/Script/Engine.Character|GetCharacterMovement (Variables|Default|GetPlayerCharacter)) 2.5e+02))))

(fn ConstructionScript)