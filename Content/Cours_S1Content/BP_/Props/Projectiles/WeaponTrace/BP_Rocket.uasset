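; BP_Rocket is a rocket projectile actor that spawns an explosion when it hits something.
; SetRocket stores a damage value and applies the given speed to the projectile movement component as both initial and maximum speed.
; The first hit, guarded by an Impact flag, spawns the explosion at the impact point, passes it a fixed radius and the rocket's location, then destroys the rocket.
; The stored damage is not passed to the explosion.
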(event Custom|Set%20Rocket
  (params (Damage :type Integer) (Speed :type Float%20%28double-precision%29))
  (Variables|Default|SetDamage Damage)
  (bind _output_get (Variables|Default|SetProjectileMovement (Variables|Default|GetProjectileMovement)))
  (bind _output_get_2 (Variables|/Script/Engine.ProjectileMovementComponent|SetInitialSpeed _output_get Speed))
  (Variables|/Script/Engine.ProjectileMovementComponent|SetMaxSpeed _output_get _output_get_2))

(event EventBeginPlay)

(event Collision|EventHit
  (params (MyComp :type Primitive%20Component%20Object%20Reference) (Other :type Actor%20Object%20Reference) (OtherComp :type Primitive%20Component%20Object%20Reference) (bSelfMoved :type Boolean) (HitLocation :type Vector :default "0, 0, 0") (HitNormal :type Vector :default "0, 0, 0") (NormalImpulse :type Vector :default "0, 0, 0") (Hit :type Hit%20Result%20Structure%20%28by%20ref%29))
  (if (not (Variables|Default|GetImpact))
    (Variables|Default|SetImpact true)
    (bind _returnvalue (Game|SpawnActorfromClass "/Game/Cours_S1Content/BP_/Props/Projectiles/Spawn_Eplosion.Spawn_Eplosion_C" (Math|Transform|MakeTransform (.ImpactPoint (Collision|BreakHitResult Hit)) "0, 0, 0" "1.000000,1.000000,1.000000") "Undefined" "MultiplyWithRoot" 0 0))
    (Default|SetExplosion _returnvalue 2e+02 (Transformation|GetActorLocation))
    (Actor|DestroyActor)))

(fn ConstructionScript)