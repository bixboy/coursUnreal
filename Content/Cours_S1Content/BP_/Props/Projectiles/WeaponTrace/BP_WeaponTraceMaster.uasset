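; BP_WeaponTraceMaster is the weapon trace projectile, named as a master, that carries damage to what it overlaps.
; SetParticle sets its damage and movement speed, and BeginPlay copies the hit bone from the player.
; After a short delay, overlap sends damage, bone, VFX location and velocity through InterfaceTakeDamage, then destroys the projectile.
; The Hit event is empty, leaving its blood-effect and damage logic disconnected.
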(event Custom|Set%20Particle
  (params (Damage :type Integer) (Speed :type Float%20%28double-precision%29))
  (Variables|Default|SetDamage Damage)
  (bind _output_get (Variables|Default|SetProjectileMovement (Variables|Default|GetProjectileMovement)))
  (bind _output_get_2 (Variables|/Script/Engine.ProjectileMovementComponent|SetInitialSpeed _output_get Speed))
  (Variables|/Script/Engine.ProjectileMovementComponent|SetMaxSpeed _output_get _output_get_2))

(event EventBeginPlay
  (|CallParentFunction)
  (bind _asbp_player (Utilities|Casting|CastToBP_Player (Game|Player|GetPlayerPawn 0)))
  (Variables|Default|SetBoneHit (Variables|/Game/Cours_S1Content/BP_/BP_Player.BP_Player_C|GetBoneHite _asbp_player)))

(event EventTick
  (params (DeltaSeconds :type Float%20%28single-precision%29))
  (|CallParentFunction DeltaSeconds) ; This node is disabled and will not be called.\nDrag off pins to build functionality.
)

(event Collision|EventHit
  (params (MyComp :type Primitive%20Component%20Object%20Reference) (Other :type Actor%20Object%20Reference) (OtherComp :type Primitive%20Component%20Object%20Reference) (bSelfMoved :type Boolean) (HitLocation :type Vector :default "0, 0, 0") (HitNormal :type Vector :default "0, 0, 0") (NormalImpulse :type Vector :default "0, 0, 0") (Hit :type Hit%20Result%20Structure%20%28by%20ref%29)))

(event Collision|EventActorBeginOverlap
  (params (OtherActor :type Actor%20Object%20Reference))
  (Utilities|FlowControl|Delay 0.1)
  (if (and (!= (Variables|Default|GetDamage) 0) (Utilities|DoesObjectImplementInterface OtherActor "/Game/Cours_S1Content/I_/InterfaceTakeDamage.InterfaceTakeDamage_C"))
    (Class|InterfaceTakeDamage|TakeDamage(Message) OtherActor (Variables|Default|GetDamage) (Variables|Default|GetBoneHit) (Transformation|GetWorldLocation (Variables|Default|GetVFX)) (Transformation|GetVelocity))
    (Actor|DestroyActor)))

(fn ConstructionScript
  (|CallParentFunction))