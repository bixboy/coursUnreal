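; Master item pickup actor that adds its item to a character's inventory when interacted with.
; InteractwithObject calls PickUp, which passes the row name and quantity from ItemDataComponent to the player's BPInventorySystem, if valid.
; It then looks up the item's data table row and, only if found, prints the item name and destroys itself.
; Replication is enabled on BeginPlay, with no authority check in the pickup logic.
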(event EventBeginPlay
  (|CallParentFunction)
  (Networking|SetReplicates true))

(event Collision|EventActorBeginOverlap
  (params (OtherActor :type Actor%20Object%20Reference))
  (|CallParentFunction OtherActor) ; This node is disabled and will not be called.\nDrag off pins to build functionality.
)

(event EventTick
  (params (DeltaSeconds :type Float%20%28single-precision%29))
  (|CallParentFunction DeltaSeconds) ; This node is disabled and will not be called.\nDrag off pins to build functionality.
)

(event EventInteractwithObject
  (params (CharacterPickingUp :type BP%20Player%20Object%20Reference))
  (CallFunction|PickUp CharacterPickingUp))

(fn ConstructionScript
  (|CallParentFunction))

(fn PickUp
  (params (Player :type BP%20Player%20Object%20Reference))
  (bind _itemdatacomponent (Variables|Default|GetItemDataComponent))
  (bind _bp_inventorysystem (Variables|/Game/Cours_S1Content/BP_/BP_Player.BP_Player_C|GetBP_InventorySystem Player))
  (bind _itemdatacomponent_2 (Variables|Default|GetItemDataComponent))
  (bind _itemid (Variables|/Game/Cours_S1Content/BP_/Inventory/ItemDataComponent.ItemDataComponent_C|GetItemID _itemdatacomponent))
  (Utilities|IsValid _bp_inventorysystem
    (:Is%20Valid
      (Default|AddtoInventory _bp_inventorysystem (.rowname (Variables|/Game/Cours_S1Content/BP_/Inventory/ItemDataComponent.ItemDataComponent_C|GetItemID _itemdatacomponent_2)) (Variables|/Game/Cours_S1Content/BP_/Inventory/ItemDataComponent.ItemDataComponent_C|GetQuantity _itemdatacomponent_2))
      (bind _returnvalue (Utilities|GetDataTableRow (.datatable _itemid) (.rowname _itemid))
        (:then
          (Development|PrintString (Utilities|String|ToString(Text) (.Name (Utilities|Struct|BreakSt_ItemInventory _returnvalue))))
          (Actor|DestroyActor))))))