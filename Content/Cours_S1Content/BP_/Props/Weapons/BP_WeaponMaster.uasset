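; BP_WeaponMaster is a base weapon Blueprint providing firing effects, fire-mode switching, reloading and scope zoom.
; Fire plays the weapon animation and ejects an impulse-driven casing, while a separate event spawns a trace projectile at the barrel, passing it damage and speed.
; Reload pairs a character montage with a weapon animation.
; Fire mode cycles semi, burst and auto when allowed, and zoom adjusts the passed camera's FOV within clamped limits.
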(event EventReloadWeapon
  (params (Mesh :type Skeletal%20Mesh%20Component%20Object%20Reference))
  (Animation|Montage|PlayMontage Mesh (Variables|Animation|GetAnimationReloadCharacter)
    (:then
      (Components|Animation|PlayAnimation (Variables|Default|GetWeaponModel) (Variables|Animation|GetAnimReload) false))))

(event EventBeginPlay
  (bind _asbp_player (Utilities|Casting|CastToBP_Player (Game|GetPlayerCharacter 0)))
  (Variables|Reference|SetPlayerRef _asbp_player)
  (Variables|Default|SetFov (Variables|Default|GetScopLenght)))

(event EventSpawnTraceBullet
  (params (Location :type Vector :default "0, 0, 0") (TraceEnd :type Vector :default "0, 0, 0"))
  (bind _returnvalue (Game|SpawnActorfromClass (Variables|Reference|GetTraceParticle) (Math|Transform|MakeTransform (Transformation|GetSocketLocation (Variables|Default|GetWeaponModel) "barrel") (Math|Rotator|FindLookatRotation Location TraceEnd)) "Undefined" "MultiplyWithRoot" 0 0))
  (Default|SetParticle _returnvalue (Variables|Default|GetDamage) 1e+04))

(event EventFire
  (bind _weaponmodel (Variables|Default|GetWeaponModel))
  (bind _returnvalue (Transformation|GetSocketRotation _weaponmodel "AmmoEject"))
  (bind (_roll _pitch _yaw) (Math|Rotator|BreakRotator _returnvalue))
  (Components|Animation|PlayAnimation (Variables|Default|GetWeaponModel) "/Game/Cours_S1Content/Animation/AnimSequence_Weapons/Fire_Pistol_W.Fire_Pistol_W" false)
  (if true
    (bind _returnvalue_2 (Game|SpawnActorfromClass (Variables|Reference|GetAmmoCasing) (Math|Transform|MakeTransform (Transformation|GetSocketLocation (Variables|Default|GetWeaponModel) "AmmoEject") (Math|Rotator|MakeRotator _roll (- _pitch 9e+01) _yaw) "0.700000,0.700000,0.700000") "Undefined" "MultiplyWithRoot" 0 0))
    (Physics|AddImpulse (Variables|/Game/Cours_S1Content/BP_/Props/Weapons/AmmoCasing_BP/BP_AmmoCasingMaster.BP_AmmoCasingMaster_C|GetBulletCasing _returnvalue_2) (+ (* (Math|Vector|GetRightVector _returnvalue) (Math|Random|RandomFloatinRange 9e+01 1.5e+02)) (* (Transformation|GetVelocity) 0.8)) "None" true)))

(event EventZoomScope
  (params (Delta%20Value :type Float%20%28double-precision%29) (CameraCaller :type Camera%20Component%20Object%20Reference))
  (bind _output_get (Variables|Default|SetFov (Math|Float|Clamp(Float) (+ (Variables|Default|GetFov) Delta%20Value) 3e+01 (Variables|Default|GetScopLenght))))
  (Camera|SetFieldOfView CameraCaller _output_get))

(event EventChangeFireMode
  (if (Variables|WeaponType|GetCanChangeFireMode?)
    (bind _output_get (Variables|Default|SetFire%20Mode (Utilities|Select :Index (Variables|Default|GetFire%20Mode) :NewEnumerator0 "NewEnumerator2" :NewEnumerator2 "NewEnumerator1" :NewEnumerator1 "NewEnumerator0")))
    (Development|PrintString (Utilities|String|EnumtoString _output_get))))

(fn ConstructionScript)