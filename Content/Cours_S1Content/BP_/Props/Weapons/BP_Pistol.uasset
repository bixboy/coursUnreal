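; BP_Pistol is a pistol weapon Blueprint that provides the cosmetic response to a Fire event.
; Fire plays the pistol's firing animation on WeaponModel and spawns a scaled-down shell casing at the AmmoEject socket.
; The casing gets a sideways impulse of random strength plus most of the actor's velocity, applied as a velocity change.
; No projectile, trace or damage logic appears here, and the other events are disabled stubs.
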(event EventBeginPlay
  (|CallParentFunction) ; This node is disabled and will not be called.\nDrag off pins to build functionality.
)

(event Collision|EventActorBeginOverlap
  (params (OtherActor :type Actor%20Object%20Reference))
  (|CallParentFunction OtherActor) ; This node is disabled and will not be called.\nDrag off pins to build functionality.
)

(event EventTick
  (params (DeltaSeconds :type Float%20%28single-precision%29))
  (|CallParentFunction DeltaSeconds) ; This node is disabled and will not be called.\nDrag off pins to build functionality.
)

(event EventFire
  (bind _weaponmodel (Variables|Default|GetWeaponModel))
  (bind _returnvalue (Transformation|GetSocketRotation _weaponmodel "AmmoEject"))
  (bind (_roll _pitch _yaw) (Math|Rotator|BreakRotator _returnvalue))
  (Components|Animation|PlayAnimation (Variables|Default|GetWeaponModel) "/Game/Cours_S1Content/Animation/AnimSequence_Weapons/Fire_Pistol_W.Fire_Pistol_W" false)
  (bind _returnvalue_2 (Game|SpawnActorfromClass (Variables|Default|GetAmmoCasing) (Math|Transform|MakeTransform (Transformation|GetSocketLocation (Variables|Default|GetWeaponModel) "AmmoEject") (Math|Rotator|MakeRotator _roll (- _pitch 9e+01) _yaw) "0.700000,0.700000,0.700000") "Undefined" "MultiplyWithRoot" 0 0))
  (Physics|AddImpulse (Variables|/Game/Cours_S1Content/BP_/Props/Weapons/AmmoCasing_BP/BP_AmmoCasingMaster.BP_AmmoCasingMaster_C|GetBulletCasing _returnvalue_2) (+ (* (Math|Vector|GetRightVector _returnvalue) (Math|Random|RandomFloatinRange 9e+01 1.5e+02)) (* (Transformation|GetVelocity) 0.8)) "None" true))

(fn ConstructionScript
  (|CallParentFunction))