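; BP_RPG is a rocket launcher weapon that extends a parent weapon Blueprint with its own firing behavior.
; Fire plays the launcher animation and ejects a casing from the AmmoEject socket, with a randomized sideways impulse plus inherited weapon velocity.
; SpawnTraceBullet spawns a BP_Rocket at the barrel socket, oriented along the given trace, and passes it the weapon's damage and a fixed speed.
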(event EventSpawnTraceBullet
  (params (Location :type Vector :default "0, 0, 0") (TraceEnd :type Vector :default "0, 0, 0"))
  (bind _returnvalue (Game|SpawnActorfromClass "/Game/Cours_S1Content/BP_/Props/Projectiles/WeaponTrace/BP_Rocket.BP_Rocket_C" (Math|Transform|MakeTransform (Transformation|GetSocketLocation (Variables|Default|GetWeaponModel) "barrel") (Math|Rotator|FindLookatRotation Location TraceEnd)) "Undefined" "MultiplyWithRoot" 0 0))
  (Default|SetRocket _returnvalue (Variables|Default|GetDamage) 5e+03))

(event EventFire
  (bind _weaponmodel (Variables|Default|GetWeaponModel))
  (bind _returnvalue (Transformation|GetSocketRotation _weaponmodel "AmmoEject"))
  (bind (_roll _pitch _yaw) (Math|Rotator|BreakRotator _returnvalue))
  (Components|Animation|PlayAnimation (Variables|Default|GetWeaponModel) "/Game/ImportEpic/MilitaryWeapSilver/Weapons/Animations/Fire_RocketLauncher_W.Fire_RocketLauncher_W" false)
  (if true
    (bind _returnvalue_2 (Game|SpawnActorfromClass (Variables|Default|GetAmmoCasing) (Math|Transform|MakeTransform (Transformation|GetSocketLocation (Variables|Default|GetWeaponModel) "AmmoEject") (Math|Rotator|MakeRotator _roll (- _pitch 9e+01) _yaw) "0.700000,0.700000,0.700000") "Undefined" "MultiplyWithRoot" 0 0))
    (Physics|AddImpulse (Variables|/Game/Cours_S1Content/BP_/Props/Weapons/AmmoCasing_BP/BP_AmmoCasingMaster.BP_AmmoCasingMaster_C|GetBulletCasing _returnvalue_2) (+ (* (Math|Vector|GetRightVector _returnvalue) (Math|Random|RandomFloatinRange 9e+01 1.5e+02)) (* (Transformation|GetVelocity) 0.8)) "None" true)))

(fn ConstructionScript
  (|CallParentFunction))