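; BP_EnemyIA is an enemy character that chases the player once PawnSensing spots them, using AI MoveTo until dead.
; Bone-specific hits subtract life and spawn blood at the struck bone; lethal ones set Dead, start ragdoll and push that bone.
; Explosion hits subtract life and always ragdoll without setting Dead, launching the pelvis with an impulse derived from the blast direction.
; The shared ragdoll function disables movement and capsule collision, then simulates physics from the pelvis down.
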(event OnSeePawn(PawnSensing)
  (params (Pawn :type Pawn%20Object%20Reference))
  (if (not (Variables|Default|GetDead?))
    (Variables|Default|SetIsSeeingPlayer? true)
    (CallFunction|FollowPlayer)))

(event Custom|Follow%20player
  (if (and (Variables|Default|GetIsSeeingPlayer?) (not (Variables|Default|GetDead?)))
    (AI|AIMoveTo self "0, 0, 0" (Game|GetPlayerCharacter 0) 7e+01 false)))

(event EventBeginPlay
  (Variables|Default|SetCurrentLife (Variables|Default|GetMaxLife)))

(event EventOnExplosionHit
  (params (Damage :type Integer) (ExplosionSource :type Vector :default "0, 0, 0"))
  (bind _returnvalue (Transformation|GetActorLocation))
  (bind _returnvalue_2 (Math|Vector|GetUnitDirection(Vector) ExplosionSource _returnvalue))
  (CallFunction|Damage Damage)
  (CallFunction|StartRagdoll)
  (Physics|AddImpulse (Variables|Character|GetMesh) (* (.x _returnvalue_2) (.y _returnvalue_2) (+ (.z _returnvalue_2) 0.1) 7e+04) "pelvis" true))

(event EventTakeDamage
  (params (Damage :type Integer) (BoneName :type Name :default "None") (AttackDirection :type Vector :default "0, 0, 0") (AttackVelocity :type Vector :default "0, 0, 0"))
  (bind _mesh (Variables|Character|GetMesh))
  (bind _returnvalue (Transformation|GetBoneTransform _mesh BoneName "RTS_World"))
  (CallFunction|Damage Damage)
  (Development|PrintString (Utilities|String|ToString(Name) BoneName))
  (Game|SpawnActorfromClass "/Game/Cours_S1Content/BP_/Props/Projectiles/Spawn_Particle_BloodDamage.Spawn_Particle_BloodDamage_C" (Math|Transform|MakeTransform (.location _returnvalue) (.rotation _returnvalue) "1.000000,1.000000,1.000000") "Undefined" "MultiplyWithRoot" 0 0)
  (if (<= (Variables|Default|GetCurrentLife) 0)
    (CallFunction|StartRagdoll)
    (Variables|Default|SetDead? true)
    (Physics|AddImpulseatLocation (Variables|Character|GetMesh) (* AttackVelocity 15.0) AttackDirection BoneName)))

(fn ConstructionScript)

(fn Damage
  (params (Damage :type Integer))
  (Variables|Default|SetCurrentLife (- (Variables|Default|GetCurrentLife) Damage))
  (Development|PrintString "hit"))

(fn StartRagdoll
  (bind _mesh (Variables|Character|GetMesh))
  (Utilities|FlowControl|Sequence
    (:then_0
      (Pawn|Components|CharacterMovement|DisableMovement (Variables|Character|GetCharacterMovement)))
    (:then_1
      (Collision|SetCollisionEnabled (Variables|Collision|GetCapsuleComponent) "NoCollision")
      (Pawn|Components|CharacterMovement|SetMovementMode (Variables|Character|GetCharacterMovement) "MOVE_None" 0)
      (Collision|SetCollisionObjectType _mesh "ECC_PhysicsBody")
      (Collision|SetCollisionEnabled _mesh "QueryAndPhysics")
      (Class|SkeletalMeshComponent|SetAllBodiesBelowSimulatePhysics (Variables|Character|GetMesh) (Utilities|Name|MakeLiteralName "pelvis") true true))))