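; Destructible oil barrel that explodes once its HP runs out.
; Each damage event removes one HP regardless of amount, and a flag ensures it explodes only once.
; At zero, it spawns an explosion actor, hides the barrel mesh and adds a Geometry Collection component with a radial impulse to scatter debris.
; The actor destroys itself after a short delay.
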(event EventBeginPlay)

(event EventTakeDamage
  (params (Damage :type Integer) (BoneName :type Name :default "None") (AttackDirection :type Vector :default "0, 0, 0") (AttackVelocity :type Vector :default "0, 0, 0"))
  (if (not (Variables|Default|GetIsExplods))
    (bind _result (Math|Integer|DecrementInt (Variables|Default|GetHP))
      (:%20%20
        (Variables|Default|SetHP _result)
        (if (<= (Variables|Default|GetHP) 0)
          (Variables|Default|SetIsExplods true)
          (bind _returnvalue (Game|SpawnActorfromClass "/Game/Cours_S1Content/BP_/Props/Projectiles/Spawn_Eplosion.Spawn_Eplosion_C" (Math|Transform|MakeTransform (Transformation|GetActorLocation) "0, 0, 0" "1.000000,1.000000,1.000000") "AlwaysSpawn" "MultiplyWithRoot" 0 0))
          (Default|SetExplosion _returnvalue 3e+02 (Transformation|GetActorLocation))
          (Rendering|SetVisibility (Variables|Default|GetBarrel) false false)
          (bind _returnvalue_2 (AddComponent|AddGeometryCollectionComponent false))
          (Physics|AddRadialImpulse _returnvalue_2 (Transformation|GetActorLocation) 2e+02 2e+02 "RIF_Constant" false)
          (Utilities|FlowControl|Delay 5.0)
          (Actor|DestroyActor))))))

(fn ConstructionScript)