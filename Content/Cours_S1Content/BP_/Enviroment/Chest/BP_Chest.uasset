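; BP_Chest is an interactable chest that opens on player interaction and closes again when something leaves its trigger area.
; The InteractwithObject event plays the open animation once on the skeletal mesh if the chest is closed.
; The Box component's end-overlap event plays the close animation, with no filter on the overlapping actor.
; An IsOpen flag gates both events so neither animation repeats out of turn.
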(event OnComponentEndOverlap(Box)
  (params (OverlappedComponent :type Primitive%20Component%20Object%20Reference) (OtherActor :type Actor%20Object%20Reference) (OtherComp :type Primitive%20Component%20Object%20Reference) (OtherBodyIndex :type Integer))
  (if (Variables|Default|GetIsOpen)
    (Components|Animation|PlayAnimation (Variables|Default|GetSkeletalMesh) "/Game/Cours_S1Content/Resources/EnvironmentAssets/Chest/anims/Chest_Anim_Armature_A_Close.Chest_Anim_Armature_A_Close" false)
    (Variables|Default|SetIsOpen false)))

(event EventInteractwithObject
  (params (CharacterPickingUp :type BP%20Player%20Object%20Reference))
  (if (not (Variables|Default|GetIsOpen))
    (Components|Animation|PlayAnimation (Variables|Default|GetSkeletalMesh) "/Game/Cours_S1Content/Resources/EnvironmentAssets/Chest/anims/Chest_Anim_Armature_A_Open.Chest_Anim_Armature_A_Open" false)
    (Variables|Default|SetIsOpen true)))

(fn ConstructionScript)