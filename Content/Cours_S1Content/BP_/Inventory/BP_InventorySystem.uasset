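; Slot-based inventory system that stores item IDs and quantities in an array sized at BeginPlay and forwards pickups to the target's interact message.
; Adding fills matching stacks up to the Item_Data table's stack size, then empty slots, returning any remainder.
; Removal and slot swaps between inventories fire an update dispatcher; adding does not.
; Dropping is unfinished: its loop is empty, the spawn is unconnected and the drop location returns zero.
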(event Custom|Serveur%20Interact
  (Class|InteractInterface|InteractwithObject(Message) (stale Custom|Pickup Target) (stale Custom|Pickup Player)))

(event Custom|Pickup
  (params (Target :type Actor%20Object%20Reference) (Player :type BP%20Player%20Object%20Reference))
  (CallFunction|ServeurInteract))

(event Custom|DropItem
  (params (ItemId :type Name) (Quantity :type Integer))
  (for _index (range 0 (- Quantity 1))
    _))

(event Custom|MCUpdate
  (Default|CallOnInventoryUpdated))

(event Custom|RemoveItem
  (params (Index :type Integer) (IsConsumed :type Boolean))
  (CallFunction|RemovefromInventory Index IsConsumed))

(event EventBeginPlay
  (Utilities|Array|Resize (Variables|Default|GetContent) (Variables|Default|GetInventorySize)))

(fn AddtoInventory
  (params (ItemID :type Name) (Quantity :type Integer))
  (LocalVariables|SetQuantity_Remaning Quantity)
  (while (and (> (LocalVariables|GetQuantity_Remaning) 0) (not (LocalVariables|GetHasFaild)))
    (bind (_index _foundslot) (CallFunction|FindSlot ItemID))
    (if _foundslot
      (CallFunction|AddtoStack _index 1)
      (Math|Integer|DecrementInt (LocalVariables|GetQuantity_Remaning))
      (elif (.HasEmptySlot (CallFunction|GetEmptySlot))
        (bind _success (CallFunction|CreatNewStack ItemID 1))
        (if _success
          (Math|Integer|DecrementInt (LocalVariables|GetQuantity_Remaning))
          (else
            (LocalVariables|SetHasFaild true)))
        (else
          (LocalVariables|SetHasFaild true)))))
  (return (not (LocalVariables|GetHasFaild)) (LocalVariables|GetQuantity_Remaning)))

(fn RemovefromInventory
  (params (Index :type Integer) (IsConsumed :type Boolean))
  (bind _content (Variables|Default|GetContent))
  (bind _content_2 (Variables|Default|GetContent))
  (bind _output (Utilities|Array|Get(acopy) _content Index))
  (bind _output_2 (Utilities|Array|Get(acopy) _content_2 Index))
  (LocalVariables|SetLocalItem (.itemid _output))
  (LocalVariables|SetLocalQuantity (.quantity _output))
  (Utilities|FlowControl|Sequence
    (:then_0
      (if (== (LocalVariables|GetLocalQuantity) 1)
        (Utilities|Array|SetArrayElem (Variables|Default|GetContent) Index (Utilities|Struct|MakeSt_SlotInventory "" 0))
        (if (not IsConsumed)
          (CallFunction|DropItem (LocalVariables|GetLocalItem) (LocalVariables|GetLocalQuantity)))
        (else
          (Utilities|Struct|SetmembersinSt_SlotInventory _output_2 (- (.Quantity (Utilities|Struct|BreakSt_SlotInventory _output_2)) 1))
          (if (not IsConsumed)
            (CallFunction|DropItem (LocalVariables|GetLocalItem) 1)))))
    (:then_1
      (CallFunction|MCUpdate))))

(fn FindSlot
  (params (ItemID :type Name))
  (for (_array_element _array_index) (Variables|Default|GetContent)
    (if (== (.ItemID (Utilities|Struct|BreakSt_SlotInventory _array_element)) ItemID)
      (if (< (.Quantity (Utilities|Struct|BreakSt_SlotInventory _array_element)) (CallFunction|GetMaxStackSize ItemID))
        (return _array_index true (.Quantity (Utilities|Struct|BreakSt_SlotInventory _array_element))))))
  (return -1 false 0))

(fn GetMaxStackSize
  (params (ItemID :type Name))
  (bind _returnvalue (Utilities|GetDataTableRow "/Game/Cours_S1Content/BP_/Inventory/Item_Data.Item_Data" ItemID)
    (:then
      (return (Utilities|Struct|BreakSt_ItemInventory _returnvalue)))
    (:RowNotFound
      (return -1))))

(fn AddtoStack
  (params (Index :type Integer) (Quantity :type Integer))
  (bind _content (Variables|Default|GetContent))
  (bind _output (Utilities|Array|Get(acopy) _content Index))
  (Utilities|Array|SetArrayElem (Variables|Default|GetContent) Index (Utilities|Struct|MakeSt_SlotInventory (.itemid _output) (+ (.quantity _output) Quantity))))

(fn GetEmptySlot
  (for (_array_element _array_index) (Variables|Default|GetContent)
    (if (== (Utilities|Struct|BreakSt_SlotInventory _array_element) 0)
      (return true _array_index)))
  (return false -1))

(fn CreatNewStack
  (params (ItemID :type Name) (Quantity :type Integer))
  (bind (_hasemptyslot _emptyindex) (CallFunction|GetEmptySlot))
  (if _hasemptyslot
    (Utilities|Array|SetArrayElem (Variables|Default|GetContent) _emptyindex (Utilities|Struct|MakeSt_SlotInventory ItemID Quantity))
    (return true)
    (else
      (return false))))

(fn Debug
  (for (_array_element _array_index) (Variables|Default|GetContent)
    (Development|PrintString (Utilities|String|Append (Utilities|String|ToString(Integer) _array_index) ":" (Utilities|String|ToString(Name) (.ItemID (Utilities|Struct|BreakSt_SlotInventory _array_element))) "=" (Utilities|String|ToString(Integer) (.Quantity (Utilities|Struct|BreakSt_SlotInventory _array_element)))))))

(fn GetItemData
  (params (itemId :type Name))
  (bind _returnvalue (Utilities|GetDataTableRow "/Game/Cours_S1Content/BP_/Inventory/Item_Data.Item_Data" itemId)
    (:then
      (return _returnvalue))))

(fn GetDropLocation
  (Collision|LineTraceByChannel "0, 0, 0" "0, 0, 0" "TraceTypeQuery1" false 0 "None")
  (return "0, 0, 0"))

(fn TransferSlots
  (params (SourceIndex :type Integer) (SourceInventory :type BP%20Inventory%20System%20Object%20Reference) (DestinationIndex :type Integer))
  (Variables|Default|SetLocalSloteConten (Utilities|Array|Get(acopy) (Variables|BP_InventorySystem_C|GetContent SourceInventory) SourceIndex))
  (if (not (< DestinationIndex 0))
    (if (not (== (.ItemID (Utilities|Struct|BreakSt_SlotInventory (Variables|Default|GetLocalSloteConten))) (.ItemID (Utilities|Struct|BreakSt_SlotInventory (Utilities|Array|Get(acopy) (Variables|Default|GetContent) DestinationIndex)))))
      (Utilities|Array|SetArrayElem (Variables|BP_InventorySystem_C|GetContent SourceInventory) SourceIndex (Utilities|Array|Get(acopy) (Variables|Default|GetContent) DestinationIndex))
      (Utilities|Array|SetArrayElem (Variables|Default|GetContent) DestinationIndex (Variables|Default|GetLocalSloteConten))
      (CallFunction|MCUpdate)
      (CallFunction|MCUpdate SourceInventory))))