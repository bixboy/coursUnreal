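; BP_Grenade is a timed grenade actor that explodes after a set delay.
; On BeginPlay its two sphere components ignore the owning actor while moving, so it does not collide with whoever threw it.
; When the TimeExplosion delay ends, Explode spawns an actor at the grenade's transform and destroys the grenade.
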(event Custom|Explode
  (Game|SpawnActorfromClass "/Game/Cours_S1Content/BP_/Props/Projectiles/Spawn_Eplosion.Spawn_Eplosion_C" (Transformation|GetActorTransform) "Undefined" "MultiplyWithRoot" 0 0)
  (Actor|DestroyActor))

(event EventBeginPlay
  (Collision|IgnoreActorwhenMoving (Variables|Default|GetSphere) (Components|GetOwner) true)
  (Utilities|FlowControl|Delay (Variables|Default|GetTimeExplosion))
  (CallFunction|Explode))

(fn ConstructionScript)