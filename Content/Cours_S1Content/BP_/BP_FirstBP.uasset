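; BP_FirstBP is an overlap-triggered moving actor, behaving like a simple lift.
; BeginPlay stores the Cube's world position as the home point.
; On overlap, MoveComponentTo eases the root to the Cube's current X and Y at LocationTarget's height plus a fixed offset.
; Ending the overlap reuses that move to return to the stored point, both over the OverTime duration.
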(event Collision|EventActorBeginOverlap
  (params (OtherActor :type Actor%20Object%20Reference))
  (bind _cube (Variables|Default|GetCube))
  (bind _returnvalue (Transformation|GetWorldLocation _cube))
  (Variables|Default|SetMoveTo (+ (Math|Vector|MakeVector (.x _returnvalue) (.y _returnvalue) 0.0) (Math|Vector|MakeVector 0.0 0.0 (+ (.z (Transformation|GetActorLocation (Variables|Default|GetLocationTarget))) 1e+02))))
  (Components|MoveComponentTo (Variables|Transformation|GetRootComponent) (Variables|Default|GetMoveTo) "0, 0, 0" true true (Variables|Default|GetOverTime) false))

(event EventBeginPlay
  (Variables|Default|SetPoseTemp (Transformation|GetWorldLocation (Variables|Default|GetCube))))

(event Collision|EventActorEndOverlap
  (params (OtherActor :type Actor%20Object%20Reference))
  (Variables|Default|SetMoveTo (Variables|Default|GetPoseTemp))
  (Components|MoveComponentTo (Variables|Transformation|GetRootComponent) (Variables|Default|GetMoveTo) "0, 0, 0" true true (Variables|Default|GetOverTime) false))

(fn ConstructionScript)